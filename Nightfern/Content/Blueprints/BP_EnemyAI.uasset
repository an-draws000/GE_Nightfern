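; BP_EnemyAI is an enemy pawn that patrols a list of waypoints and chases the player once seen.
; From BeginPlay, Roam chains AI MoveTo calls, advancing the waypoint index on each success and wrapping to the start.
; PawnSensing sets a seen flag that is never cleared here and issues one move toward the player character.
; Failed moves are not handled, so an interrupted patrol does not resume.
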(event OnSeePawn(PawnSensing)
  (params (Pawn :type Pawn%20Object%20Reference))
  (Variables|Default|SetIsSeingPlayer true)
  (CallFunction|FollowPlayer))

(event Custom|FollowPlayer
  (if (Variables|Default|GetIsSeingPlayer)
    (AI|AIMoveTo self "0, 0, 0" (Game|GetPlayerCharacter 0) 5.0 false)))

(event Custom|Roam
  (AI|AIMoveTo self "0, 0, 0" (Utilities|Array|Get(acopy) (Variables|Default|GetWaypoints) (Variables|Default|GetCurrentIndex)) 5.0 false
    (:OnSuccess
      (bind _result (Math|Integer|IncrementInt (Variables|Default|GetCurrentIndex))
        (:%20%20
          (if (>= _result (Utilities|Array|Length (Variables|Default|GetWaypoints)))
            (Variables|Default|SetCurrentIndex 0)
            (CallFunction|Roam)
            (else
              (CallFunction|Roam))))))))

(event EventBeginPlay
  (CallFunction|Roam))

(fn ConstructionScript)