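; BP_EnemyHealth is a health component that tracks current and maximum HP for its owning actor.
; IncreaseMaxHP sets the maximum to a base plus increment and refills HP, without updating the bar.
; DecreaseHP returns true on lethal damage without lowering HP, while IncreaseHP rejects heals beyond the maximum instead of clamping.
; Despite the enemy name, successful changes update the HUD bar by casting the owner to BP_TopDownCharacter.
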(event EventBeginPlay)

(fn IncreaseMaxHP
  (params (Incremention :type Float%20%28double-precision%29))
  (bind _output_get (Variables|Default|SetMaxHP (+ 1e+02 Incremention)))
  (Variables|Default|SetCurrentHP _output_get))

(fn DecreaseHP
  (params (Damage :type Float%20%28double-precision%29))
  (if (> (- (Variables|Default|GetCurrentHP) Damage) 0.0)
    (Variables|Default|SetCurrentHP (- (Variables|Default|GetCurrentHP) Damage))
    (bind _asbp_top_down_character (Utilities|Casting|CastToBP_TopDownCharacter (Components|GetOwner)))
    (Progress|SetPercent (Variables|/Game/UI/WB_HUD.WB_HUD_C|GetHPBar (Variables|/Game/Blueprints/BP_TopDownCharacter.BP_TopDownCharacter_C|GetHUD%20Widget _asbp_top_down_character)) (/ (Variables|Default|GetCurrentHP) (Variables|Default|GetMaxHP)))
    (return false)
    (else
      (Development|PrintString "Dead ass")
      (return true))))

(fn IncreaseHP
  (params (Heal :type Float%20%28double-precision%29))
  (if (<= (+ (Variables|Default|GetCurrentHP) Heal) (Variables|Default|GetMaxHP))
    (Variables|Default|SetCurrentHP (+ (Variables|Default|GetCurrentHP) Heal))
    (bind _asbp_top_down_character (Utilities|Casting|CastToBP_TopDownCharacter (Components|GetOwner)))
    (Progress|SetPercent (Variables|/Game/UI/WB_HUD.WB_HUD_C|GetHPBar (Variables|/Game/Blueprints/BP_TopDownCharacter.BP_TopDownCharacter_C|GetHUD%20Widget _asbp_top_down_character)) (/ (Variables|Default|GetCurrentHP) (Variables|Default|GetMaxHP)))
    (else
      (Development|PrintString "Nuh uh"))))