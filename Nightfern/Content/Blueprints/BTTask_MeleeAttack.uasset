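; Behavior tree task that makes an enemy perform a melee attack on the blackboard's player character.
; If the target is within range, it plays an attack montage and starts a timer; otherwise it fails.
; The timer fires a short forward sphere trace with debug drawing, ignoring the enemy.
; A hit sends damage through ApplyHitMessage and succeeds, while a miss never calls FinishExecute.
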(event Custom|Attack
  (bind (_outhit _returnvalue) (Collision|SphereTraceByChannel (Transformation|GetActorLocation (stale EventReceiveExecuteAI _asbp_enemy_base)) (+ (Transformation|GetActorLocation (stale EventReceiveExecuteAI _asbp_enemy_base)) (* (Transformation|GetActorForwardVector (stale EventReceiveExecuteAI _asbp_enemy_base)) 8e+01)) 8e+01 "TraceTypeQuery1" false (Variables|Default|GetActors%20to%20Ignore) "ForDuration"))
  (if _returnvalue
    (Class|BPIDamageable|ApplyHit(Message) (.hitactor _outhit) 15.0)
    (AI|BehaviorTree|FinishExecute true)))

(event EventReceiveExecuteAI
  (params (OwnerController :type AI%20Controller%20Object%20Reference) (ControlledPawn :type Pawn%20Object%20Reference))
  (Utilities|Array|Add (Variables|Default|GetActors%20to%20Ignore) ControlledPawn)
  (bind _asbp_enemy_base (Utilities|Casting|CastToBP_EnemyBase ControlledPawn))
  (bind _asbp_top_down_character (Utilities|Casting|CastToBP_TopDownCharacter (AI|Components|Blackboard|GetValueasObject (AI|GetBlackboard OwnerController) (Variables|Default|GetKey%20Name))))
  (if (<= (Transformation|GetDistanceTo _asbp_enemy_base _asbp_top_down_character) 1.8e+02)
    (Animation|PlayAnimMontage _asbp_enemy_base "/Game/Animations/EnemyAnimation/EnemyMelee_Attack_AnimMontage.EnemyMelee_Attack_AnimMontage" 1.0 "None")
    (Utilities|Time|SetTimerbyEvent (delegate Custom|Attack) 0.85)
    (else
      (AI|BehaviorTree|FinishExecute false))))