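; GI_Nightfern is a game instance that sends the player through rooms in random order and tracks the current level count.
; LoadNextRoom picks a random template name, records it as used, increments CurrentLevel and opens that level.
; The removed index is rolled separately, so it can differ from the chosen room.
; The MainMenu fallback is unreachable because the length check against -1 always passes.
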(event EventInit)

(fn LoadNextRoom
  (bind _availableroomtemplates (Variables|Default|GetAvailableRoomTemplates))
  (bind _availableroomtemplates_2 (Variables|Default|GetAvailableRoomTemplates))
  (bind _returnvalue (Utilities|Array|Length _availableroomtemplates))
  (LocalVariables|SetavailableRooms _returnvalue)
  (if (> _returnvalue -1)
    (bind _output_get (LocalVariables|SetRoomName (Utilities|Array|Get(acopy) _availableroomtemplates_2 (Math|Random|RandomIntegerinRange 0 (- (LocalVariables|GetavailableRooms) 1)))))
    (Utilities|Array|Add (Variables|Default|GetUsedRoomTemplates) _output_get)
    (Utilities|Array|RemoveIndex _availableroomtemplates_2 (Math|Random|RandomIntegerinRange 0 (- (LocalVariables|GetavailableRooms) 1)))
    (bind _result (Math|Integer|IncrementInt (Variables|Default|GetCurrentLevel))
      (:%20%20
        (Variables|Default|SetCurrentLevel _result)
        (Game|OpenLevel(byName) (LocalVariables|GetRoomName))))
    (else
      (Game|OpenLevel(byObjectReference) "/Game/Maps/MainMenu.MainMenu"))))