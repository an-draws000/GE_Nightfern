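; AI controller for enemy pawns that runs their behavior and tracks the player character through perception.
; On possessing a BP_EnemyBase, it sets up the BB_Enemy blackboard and runs the behavior tree asset stored on that enemy, so each enemy can supply its own tree.
; AI Perception updates write a sensed BP_TopDownCharacter to a blackboard key and clear that key when sensing fails.
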(event OnTargetPerceptionUpdated(AIPerception)
  (params (Actor :type Actor%20Object%20Reference) (Stimulus :type AI%20Stimulus%20Structure))
  (bind _returnvalue (AI|GetBlackboard 0))
  (bind _key_name (Variables|Default|GetKey%20Name))
  (Utilities|Casting|CastToBP_TopDownCharacter Actor)
  (if (.bSuccessfullySensed (Utilities|Struct|BreakAIStimulus Stimulus))
    (AI|Components|Blackboard|SetValueasObject _returnvalue _key_name Actor)
    (else
      (AI|Components|Blackboard|ClearValue _returnvalue _key_name))))

(event EventBeginPlay)

(event EventTick
  (params (DeltaSeconds :type Float%20%28single-precision%29)))

(event EventPossess
  (params (PossessedPawn :type Pawn%20Object%20Reference))
  (bind _asbp_enemy_base (Utilities|Casting|CastToBP_EnemyBase PossessedPawn))
  (Class|AIController|UseBlackboard "/Game/Blueprints/BB_Enemy.BB_Enemy")
  (AI|RunBehaviorTree (Variables|/Game/Blueprints/BP_EnemyBase.BP_EnemyBase_C|GetBehaviorTreeAsset _asbp_enemy_base)))

(fn ConstructionScript)