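; BP_RoomManager moves the game to a randomly picked room level shortly after play begins.
; After a brief delay, LoadRandomRoom copies an entry from GI_Nightfern's AvailableRoomTemplates into UsedRoomTemplates, removes one, then opens one by name.
; The game instance holds both lists, so they persist across level loads.
; Each step rolls its own random index, so the recorded, removed and opened rooms can differ.
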(event EventBeginPlay
  (Utilities|FlowControl|Delay 0.5)
  (CallFunction|LoadRandomRoom))

(event Collision|EventActorBeginOverlap
  (params (OtherActor :type Actor%20Object%20Reference)))

(event EventTick
  (params (DeltaSeconds :type Float%20%28single-precision%29)))

(fn ConstructionScript)

(fn LoadRandomRoom
  (bind _asgi_nightfern (Utilities|Casting|CastToGI_Nightfern (Game|GetGameInstance)))
  (Utilities|Array|Add (Variables|/Game/Blueprints/GI_Nightfern.GI_Nightfern_C|GetUsedRoomTemplates _asgi_nightfern) (Utilities|Array|Get(acopy) (Variables|/Game/Blueprints/GI_Nightfern.GI_Nightfern_C|GetAvailableRoomTemplates _asgi_nightfern) (Math|Random|RandomIntegerinRange 0 (- (Utilities|Array|Length (Variables|/Game/Blueprints/GI_Nightfern.GI_Nightfern_C|GetAvailableRoomTemplates _asgi_nightfern)) 1))))
  (Utilities|Array|RemoveIndex (Variables|/Game/Blueprints/GI_Nightfern.GI_Nightfern_C|GetAvailableRoomTemplates _asgi_nightfern) (Math|Random|RandomIntegerinRange 0 (- (Utilities|Array|Length (Variables|/Game/Blueprints/GI_Nightfern.GI_Nightfern_C|GetAvailableRoomTemplates _asgi_nightfern)) 1)))
  (Game|OpenLevel(byName) (Utilities|Array|Get(acopy) (Variables|/Game/Blueprints/GI_Nightfern.GI_Nightfern_C|GetAvailableRoomTemplates _asgi_nightfern) (Math|Random|RandomIntegerinRange 0 (- (Utilities|Array|Length (Variables|/Game/Blueprints/GI_Nightfern.GI_Nightfern_C|GetAvailableRoomTemplates _asgi_nightfern)) 1)))))