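; Base enemy Blueprint that takes damage, dies and spots the player's top-down character for its AI.
; On BeginPlay it seeds the BPEnemyHealth component from its MaxHP, and ApplyHit passes damage to that component, destroying the actor when it reports death.
; PawnSensing writes the seen BP_TopDownCharacter to the BP_EnemyAIController's blackboard only while that key holds no valid object.
; Current HP is debug-printed at start and after each hit.
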(event OnSeePawn(PawnSensing)
  (params (Pawn :type Pawn%20Object%20Reference))
  (bind _key_name (Variables|Default|GetKey%20Name))
  (bind _asbp_top_down_character (Utilities|Casting|CastToBP_TopDownCharacter Pawn))
  (bind _asbp_enemy_aicontroller (Utilities|Casting|CastToBP_EnemyAIController (Pawn|GetController)))
  (if (not (Utilities|IsValid (AI|Components|Blackboard|GetValueasObject (AI|GetBlackboard _asbp_enemy_aicontroller) _key_name)))
    (AI|Components|Blackboard|SetValueasObject (AI|GetBlackboard _asbp_enemy_aicontroller) _key_name _asbp_top_down_character)))

(event EventBeginPlay
  (bind _bp_enemyhealth (Variables|Default|GetBP_EnemyHealth))
  (bind _output_get (Variables|/Game/Blueprints/BP_EnemyHealth.BP_EnemyHealth_C|SetMaxHP _bp_enemyhealth (Variables|Default|GetMaxHP)))
  (bind _output_get_2 (Variables|/Game/Blueprints/BP_EnemyHealth.BP_EnemyHealth_C|SetCurrentHP _bp_enemyhealth _output_get))
  (Development|PrintString (Utilities|String|ToString(Float) _output_get_2)))

(event EventApplyHit
  (params (Damage :type Float%20%28double-precision%29))
  (bind _bp_enemyhealth (Variables|Default|GetBP_EnemyHealth))
  (bind _isdead (Default|DecreaseHP _bp_enemyhealth Damage))
  (bind _output_get (Variables|Default|SetisDead _isdead))
  (Development|PrintString (Utilities|String|ToString(Float) (Variables|/Game/Blueprints/BP_EnemyHealth.BP_EnemyHealth_C|GetCurrentHP _bp_enemyhealth)))
  (if _output_get
    (Actor|DestroyActor)))

(fn ConstructionScript)