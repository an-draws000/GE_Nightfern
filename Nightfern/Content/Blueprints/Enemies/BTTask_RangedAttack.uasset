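; Behavior Tree task that makes an enemy fire a projectile at the player character stored in a blackboard key.
; It turns the BP_EnemyBase pawn toward the target, plays the melee attack montage sped up, and spawns BP_Projectile near the pawn aimed at the target.
; It finishes successfully without waiting for the montage, but a failed cast stops it without calling FinishExecute.
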(event EventReceiveExecuteAI
  (params (OwnerController :type AI%20Controller%20Object%20Reference) (ControlledPawn :type Pawn%20Object%20Reference))
  (bind _returnvalue (Transformation|GetActorLocation ControlledPawn))
  (bind _asbp_top_down_character (Utilities|Casting|CastToBP_TopDownCharacter (AI|Components|Blackboard|GetValueasObject (AI|GetBlackboard OwnerController) (Variables|Default|GetKey%20Name))))
  (bind _asbp_enemy_base (Utilities|Casting|CastToBP_EnemyBase ControlledPawn))
  (Transformation|SetActorRotation _asbp_enemy_base (Math|Rotator|FindLookatRotation _returnvalue (Transformation|GetActorLocation _asbp_top_down_character)))
  (Animation|PlayAnimMontage _asbp_enemy_base "/Game/Animations/EnemyAnimation/EnemyMelee_Attack_AnimMontage.EnemyMelee_Attack_AnimMontage" 1.5 "None")
  (Game|SpawnActorfromClass "/Game/Blueprints/Enemies/BP_Projectile.BP_Projectile_C" (Math|Transform|MakeTransform (- _returnvalue 1e+01) (Math|Rotator|FindLookatRotation _returnvalue (Transformation|GetActorLocation _asbp_top_down_character)) "1.000000,1.000000,1.000000") "Undefined" "MultiplyWithRoot" 0 0)
  (AI|BehaviorTree|FinishExecute true))