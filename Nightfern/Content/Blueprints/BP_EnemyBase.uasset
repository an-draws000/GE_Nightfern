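; BP_EnemyBase is an enemy Blueprint, named as a base, that tracks hit points and death state.
; It delegates health to BPEnemyHealth, seeding that object's max and current HP from its own MaxHP on BeginPlay.
; ApplyHit passes damage to DecreaseHP and stores the result in IsDead, with no death reaction in this graph.
; Both events print current HP for debugging.
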(event EventBeginPlay
  (bind _bp_enemyhealth (Variables|Default|GetBP_EnemyHealth))
  (bind _output_get (Variables|/Game/Blueprints/BP_EnemyHealth.BP_EnemyHealth_C|SetMaxHP _bp_enemyhealth (Variables|Default|GetMaxHP)))
  (bind _output_get_2 (Variables|/Game/Blueprints/BP_EnemyHealth.BP_EnemyHealth_C|SetCurrentHP _bp_enemyhealth _output_get))
  (Development|PrintString (Utilities|String|ToString(Float) _output_get_2)))

(event EventApplyHit
  (params (Damage :type Float%20%28double-precision%29))
  (bind _bp_enemyhealth (Variables|Default|GetBP_EnemyHealth))
  (bind _isdead (Default|DecreaseHP _bp_enemyhealth Damage))
  (Variables|Default|SetisDead _isdead)
  (Development|PrintString (Utilities|String|ToString(Float) (Variables|/Game/Blueprints/BP_EnemyHealth.BP_EnemyHealth_C|GetCurrentHP _bp_enemyhealth))))

(fn ConstructionScript)