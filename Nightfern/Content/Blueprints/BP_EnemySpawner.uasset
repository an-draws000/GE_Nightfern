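; BP_EnemySpawner is an actor that spawns a random group of enemies around itself when play begins.
; The upper bound of the random spawn count grows with CurrentLevel from the GI_Nightfern game instance, and nothing spawns if that cast fails.
; Each enemy class is picked at random from EnemyClasses and placed at a random horizontal offset within a square centered on the spawner.
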(event EventBeginPlay
  (bind _asgi_nightfern (Utilities|Casting|CastToGI_Nightfern (Game|GetGameInstance)))
  (for _index (range 0 (Math|Random|RandomIntegerinRange 1 (+ (Variables|/Game/Blueprints/GI_Nightfern.GI_Nightfern_C|GetCurrentLevel _asgi_nightfern) 1)))
    (Game|SpawnActorfromClass (.OutItem (Utilities|Array|Random (Variables|Default|GetEnemyClasses))) (Math|Transform|MakeTransform (+ (Transformation|GetActorLocation) (Math|Vector|MakeVector (Math|Random|RandomFloatinRange -3e+02 3e+02) (Math|Random|RandomFloatinRange -3e+02 3e+02) 0.0)) "0, 0, 0" "1.000000,1.000000,1.000000") "Undefined" "MultiplyWithRoot" 0 0)))

(event Collision|EventActorBeginOverlap
  (params (OtherActor :type Actor%20Object%20Reference)))

(event EventTick
  (params (DeltaSeconds :type Float%20%28single-precision%29)))

(fn ConstructionScript)