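; BP_Dummy is a damageable dummy actor that tracks hit points through its BPEnemyHealth member.
; BeginPlay copies the dummy's MaxHP into that health object as both maximum and current HP, then prints the value.
; ApplyHit passes damage to DecreaseHP, destroying the actor when it returns true and printing the current HP otherwise.
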(event EventBeginPlay
  (bind _bp_enemyhealth (Variables|Default|GetBP_EnemyHealth))
  (Variables|/Game/Blueprints/BP_EnemyHealth.BP_EnemyHealth_C|SetMaxHP _bp_enemyhealth (Variables|Default|GetMaxHP))
  (Variables|/Game/Blueprints/BP_EnemyHealth.BP_EnemyHealth_C|SetCurrentHP _bp_enemyhealth (Variables|Default|GetMaxHP))
  (Development|PrintString (Utilities|String|ToString(Float) (Variables|/Game/Blueprints/BP_EnemyHealth.BP_EnemyHealth_C|GetCurrentHP _bp_enemyhealth))))

(event EventApplyHit
  (params (Damage :type Float%20%28double-precision%29))
  (bind _bp_enemyhealth (Variables|Default|GetBP_EnemyHealth))
  (bind _isdead (Default|DecreaseHP _bp_enemyhealth Damage))
  (if _isdead
    (Actor|DestroyActor)
    (else
      (Development|PrintString (Utilities|String|ToString(Float) (Variables|/Game/Blueprints/BP_EnemyHealth.BP_EnemyHealth_C|GetCurrentHP _bp_enemyhealth))))))

(fn ConstructionScript)